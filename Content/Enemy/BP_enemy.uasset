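; BP_enemy is an enemy actor that fires when it senses a pawn and is destroyed by bullets.
; PawnSensing sets a seeing flag and calls Shoot, which waits on a delay, spawns a BP_Bullet at the Scene component's transform and calls ApplyDamage with no target set.
; Overlapping any BP_Bullet destroys the enemy outright.
; The seeing flag is never cleared, and several unconnected debug and soldier-health nodes never run.
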(event OnSeePawn(PawnSensing)
  (params (Pawn :type Pawn%20Object%20Reference))
  (Variables|Default|SetISseeingplayer true)
  (CallFunction|Shoot))

(event Custom|shoot
  (bind _scene (Variables|Default|GetScene))
  (bind _returnvalue (Transformation|GetWorldTransform _scene))
  ;[0.15 0.15 0.15 0.5] shooting
  (if (Variables|Default|GetISseeingplayer)
    (Utilities|FlowControl|Delay 3.0)
    (Game|SpawnActorfromClass "/Game/bullet/BP_Bullet.BP_Bullet_C" (Math|Transform|MakeTransform (.location _returnvalue) (.rotation _returnvalue) "1.000000,1.000000,1.000000") "Undefined" "MultiplyWithRoot" 0 0)
    (Game|Damage|ApplyDamage 0 1.0 0 0)))

(event EventBeginPlay)

(event EventTick
  (params (DeltaSeconds :type Float%20%28single-precision%29)))

(event Collision|EventActorBeginOverlap
  (params (OtherActor :type Actor%20Object%20Reference))
  (Utilities|Casting|CastToBP_Bullet OtherActor)
  (Actor|DestroyActor))

(fn ConstructionScript)